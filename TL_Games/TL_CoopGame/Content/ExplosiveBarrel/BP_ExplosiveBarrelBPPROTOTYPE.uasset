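; Prototype explosive barrel that explodes when it takes point damage and its SHealth component's health is below one.
; Each hit draws a debug marker and damage value; the explosion deals full radial damage from the hit location, not the barrel's center.
; It also draws the blast radius, swaps to an exploded material and pushes its own mesh with radial force.
; No flag prevents later hits from re-triggering the explosion.
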(event Game|Damage|EventPointDamage
  (params (Damage :type Float%20%28single-precision%29) (DamageType :type Damage%20Type%20Object%20Reference) (HitLocation :type Vector :default "0, 0, 0") (HitNormal :type Vector :default "0, 0, 0") (HitComponent :type Primitive%20Component%20Object%20Reference) (BoneName :type Name :default "None") (ShotFromDirection :type Vector :default "0, 0, 0") (InstigatedBy :type Controller%20Object%20Reference) (DamageCauser :type Actor%20Object%20Reference) (HitInfo :type Hit%20Result%20Structure%20%28by%20ref%29))
  (bind _explosivebarreldamage (Variables|Default|GetExplosiveBarrelDamage))
  (bind _explsivebarrelradius (Variables|Default|GetExplsiveBarrelRadius))
  (bind _output_get (Variables|Default|SetDamageAppliedLocation HitLocation))
  (Rendering|Debug|DrawDebugSphere _output_get 5.0 12 "(R=0.218750,G=0.013255,B=0.006726,A=1.000000)" 1.0 1.0)
  (Rendering|Debug|DrawDebugString _output_get (Utilities|String|ToString(Float) Damage) 0 "(R=1.000000,G=1.000000,B=1.000000,A=1.000000)" 1.0)
  (if (CallFunction|IsDamaged)
    (Game|Damage|ApplyRadialDamage _explosivebarreldamage (Variables|Default|GetDamageAppliedLocation) _explsivebarrelradius 0 0 0 0 true "ECC_Visibility")
    (Rendering|Debug|DrawDebugSphere (Variables|Default|GetDamageAppliedLocation) _explsivebarrelradius 12 "(R=0.218750,G=0.013255,B=0.006726,A=1.000000)" 2.0 1.0)
    (Rendering|Material|SetMaterial (Variables|Default|GetStaticMesh) 0 "/Game/ExplosiveBarrel/M_ExplosiveBarrelExploded.M_ExplosiveBarrelExploded")
    (Physics|AddRadialForce (Variables|Default|GetStaticMesh) (Variables|Default|GetDamageAppliedLocation) _explsivebarrelradius _explosivebarreldamage "RIF_Constant" false)))

(fn ConstructionScript)

(fn IsDamaged
  (return (< (Variables|/Script/TL_CoopGame.SHealthComponent|GetHealth (Variables|Default|GetSHealth)) 1.0)))